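; BP_Character is a side-scrolling player character with left/right movement, jumping and an attack, animated through a PaperZD-style animation instance.
; Axis inputs add movement along world X, with Move_Right also setting the IsMovingright facing flag.
; Attack input jumps the animation to Attack_1, while jumping and walking off ledges both jump it to InitJump.
; The HandleRotation function is an empty stub.
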(event `InputAxis|Move_Right`
  (params (AxisValue :type "Float (single-precision)"))
  ;[1 0.16 0.16] Left Right Movement
  (if (> AxisValue 0.0)
    (set `self.isMovingright` true)
    (elif (< AxisValue 0.0)
      (set `self.isMovingright` false)))
  (`self.AddMovementInput` (1.0 0.0 0.0) AxisValue))

(event `InputAxis|Move_Left`
  (params (AxisValue :type "Float (single-precision)"))
  ;[1 0.16 0.16] Left Right Movement
  (`self.AddMovementInput` (2.0 0.0 0.0) AxisValue))

(event `InputAction|Jump`
  (params (Key :type "Key Structure"))
  ;[1 1 1] Jumping and animation handling
  (:`Pressed`
    (`self.Jump`)))

(event `InputAction|Attack_1`
  (params (Key :type "Key Structure"))
  (:`Pressed`
    (`PaperZDAnimInstance.JumpToNode` (`PaperZDAnimationComponent.AnimInstance` (`self.AnimationComponent`)) "Attack_1" "None")))

(event `self.OnJumped`
  ;[1 1 1] Jumping and animation handling
  (`PaperZDAnimInstance.JumpToNode` (`PaperZDAnimationComponent.AnimInstance` (`self.AnimationComponent`)) "InitJump" "None" :!label _label))

(event `self.OnWalkingOffLedge`
  (params (PreviousFloorImpactNormal :type "Vector Structure (by ref)") (PreviousFloorContactNormal :type "Vector Structure (by ref)") (PreviousLocation :type "Vector Structure (by ref)") (TimeDelta :type "Float (single-precision)"))
  ;[1 1 1] Jumping and animation handling
  (goto _label))

(fn `Handle Rotation`)

(fn `UserConstructionScript`)